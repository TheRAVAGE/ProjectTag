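; BP_MainLvl_GameMode is the main level's game mode Blueprint, and its graphs here contain only debug display logic.
; On Tick, when ShowDebugMessages is set, it calls two helpers, each gated by its own flag.
; DebugPlayerRole prints every name and role in PlayerRoleMap as one string, while DebugMatchState prints CustomMatchState.
; Both prints use fixed keys, so on-screen messages update in place instead of stacking.
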(event EventTick
  (params (DeltaSeconds :type Float%20%28single-precision%29))
  (Utilities|FlowControl|Sequence
    (:then_0
      (if (Variables|Default|GetbShowDebugMessages)
        (CallFunction|DebugPlayerRole)
        (CallFunction|DebugMatchState)))))

(fn ConstructionScript)

(fn DebugPlayerRole
  (if (Variables|Default|GetbShowRoleDebug)
    (LocalVariables|SetDebugString "RoleMap : 
")
    (bind (_keypin _valuepin) (Utilities|Map|ForEachLoop(Map) (Variables|Default|GetPlayerRoleMap))
      (:then
        (LocalVariables|SetDebugString (Utilities|String|Append (LocalVariables|GetDebugString) (Utilities|String|ToString(Text) (Utilities|Text|FormatText "Name: {Name}, Role : {Role} 
" _keypin (Utilities|String|EnumtoString _valuepin))))))
      (:CompletedPin
        (Development|PrintString (LocalVariables|GetDebugString) true true "(R=0.000000,G=0.660000,B=1.000000,A=1.000000)" 2.0 "RoleMap")))))

(fn DebugMatchState
  (bind _returnvalue (Utilities|String|MakeLiteralString "Match State"))
  (if (Variables|Default|GetbShowMatchStateDebug)
    (Development|PrintString (Utilities|String|Append _returnvalue " : " (Utilities|String|EnumtoString (Variables|Default|GetCustomMatchState))) true true "(R=0.000000,G=0.660000,B=1.000000,A=1.000000)" 2.0 (Utilities|String|StringToName _returnvalue))))