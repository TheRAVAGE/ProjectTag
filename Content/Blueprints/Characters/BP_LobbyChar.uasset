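; Lobby player character Blueprint that handles replicated idle-break and traversal montages, plus temporary debug keys for quitting and slow motion.
; Idle breaks are chosen on the server via chooser and random pose search database entry, then multicast.
; Traversal uses a chooser and motion matching on the locally controlled client, plays immediately, then replicates through server and multicast.
; Traversal playback sets warp targets, flying movement, obstacle collision ignore and a gameplay tag until completion.
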(event Custom|Server_PlayEvaluateIdleBreak
  ;[0 0 0 0.5] Perform Idle Break
  (bind _asabp_main_player (Utilities|Casting|CastToABP_MainPlayer (Components|SkeletalMesh|GetAnimInstance (Variables|Default|GetCharacterMesh))))
  (bind _result (|EvaluateChooser2 _asabp_main_player)
    (:execute
      (bind _object (Utilities|AsyncLoadAsset _result)
        (:Completed
          (bind _aspose_search_database (Utilities|Casting|CastToPoseSearchDatabase _object))
          (bind _asanim_montage (Utilities|Casting|CastToAnimMontage (Class|PoseSearchDatabase|GetAnimationAsset _aspose_search_database (Math|Random|RandomInteger (Class|PoseSearchDatabase|GetNumAnimationAssets _aspose_search_database)))))
          (bind _output_get (Variables|Default|SetCurrentlyPlaying_IdleAnimMontage _asanim_montage))
          (CallFunction|MCPlayIdleBreaks _output_get))))))

(event Custom|MC_PlayIdleBreaks
  (params (Idle%20Break%20Anim%20Montage :type Anim%20Montage%20Object%20Reference))
  ;[0 0 0 0.5] Perform Idle Break
  (Animation|Montage|PlayMontage (Variables|Default|GetCharacterMesh) Idle%20Break%20Anim%20Montage
    (:OnCompleted
      (Class|PlayerCharacter|ServerPerformIdleBreakTimerChecks)
      (Variables|Default|SetbShouldPerformIdleBreak false))
    (:OnBlendOut
      (Variables|Default|SetbShouldPerformIdleBreak false :!label _label))
    (:OnInterrupted
      (goto _label))
    (:OnNotifyEnd
      (goto _label))))

(event Custom|MC_PerformTraversal
  (params (TraversalCheckResults :type Traversal%20Check%20Results%20Structure))
  ;[0.15 0.005283 0 0.5] Traversal
  (if (not (Pawn|IsLocallyControlled))
    (CallFunction|PerformTraversal TraversalCheckResults)))

(event Custom|Server_PerformTraversal
  (params (TraversalCheckResults :type Traversal%20Check%20Results%20Structure))
  ;[0.15 0.005283 0 0.5] Traversal
  (CallFunction|MCPerformTraversal TraversalCheckResults))

(event Custom|PerformTraversal
  (params (TraversalCheckResults :type Traversal%20Check%20Results%20Structure))
  (bind (_traversalactor _chosenmontage _starttime _playrate) (Utilities|Struct|BreakTraversalCheckResults TraversalCheckResults))
  (bind _traversalcomp (Variables|Default|GetTraversalComp))
  (bind _charactermovementcomp (Variables|Default|GetCharacterMovementComp))
  (bind _capsulecomp (Variables|Default|GetCapsuleComp))
  ;[0.15 0.005283 0 0.5] Traversal
  (Animation|Montage|PlayMontage (Variables|Default|GetCharacterMesh) _chosenmontage _playrate _starttime
    (:then
      (Class|TraversalComponent|SetWarpTargetsforTraversal _traversalcomp TraversalCheckResults)
      (Pawn|Components|CharacterMovement|SetMovementMode _charactermovementcomp "MOVE_Flying" 0)
      (Class|PlayerCharacter|SetReplicationBehaviour true)
      (Collision|IgnoreActorwhenMoving _capsulecomp _traversalactor true)
      (Class|PlayerCharacter|ServerAddGameplayTag "(TagName=\"Tag.Player.Status.Action.Traversal\")")
      (Class|TraversalInterface|SetTraversingCharacter(Message) _traversalactor self))
    (:OnCompleted
      (Class|TraversalComponent|RemoveWarpTargetsforTraversal _traversalcomp :!label _label)
      (Pawn|Components|CharacterMovement|SetMovementMode _charactermovementcomp "MOVE_Walking" 0)
      (Class|PlayerCharacter|SetReplicationBehaviour false)
      (Collision|ClearMoveIgnoreActors _capsulecomp)
      (Class|TraversalComponent|TraversalCompleted (Variables|Default|GetTraversalComp))
      (Class|PlayerCharacter|ServerRemoveGameplayTag "(TagName=\"Tag.Player.Status.Action.Traversal\")" false)
      (Class|TraversalInterface|SetTraversingCharacter(Message) _traversalactor))
    (:OnBlendOut
      (goto _label))
    (:OnInterrupted
      (goto _label))))

(event EventBlueprintPerformIdleBreak
  ;[0 0 0 0.5] Perform Idle Break
  (CallFunction|ServerPlayEvaluateIdleBreak))

(event EventBlueprintEvaluateTraversal
  (params (AnimInstance :type Main%20Anim%20Instance%20Object%20Reference) (TraversalCheckResults :type Traversal%20Check%20Results%20Structure))
  ;[0.15 0.005283 0 0.5] Traversal
  (if (Pawn|IsLocallyControlled)
    (bind (_traversalcheckresults _result) (|EvaluateChooser2 AnimInstance TraversalCheckResults)
      (:execute
        (bind _object (Utilities|AsyncLoadAsset _result)
          (:Completed
            (bind _aspose_search_database (Utilities|Casting|CastToPoseSearchDatabase _object))
            (bind _asanim_montage (Utilities|Casting|CastToAnimMontage (.selectedanim (Class|PoseSearchLibrary|MotionMatch AnimInstance (Utilities|Array|MakeArray _aspose_search_database) "PoseHistory")))
              (:then
                (bind _structout (Utilities|Struct|SetmembersinTraversalCheckResults (Utilities|Struct|MakeTraversalCheckResults (.TraversableType (Utilities|Struct|BreakTraversalCheckResults _traversalcheckresults)) (.DistanceToTraversalObject (Utilities|Struct|BreakTraversalCheckResults _traversalcheckresults)) (.bHasFrontLedge (Utilities|Struct|BreakTraversalCheckResults _traversalcheckresults)) (.FrontLedgeLocation (Utilities|Struct|BreakTraversalCheckResults _traversalcheckresults)) (.FrontLedgeNormal (Utilities|Struct|BreakTraversalCheckResults _traversalcheckresults)) (.bHasBackLedge (Utilities|Struct|BreakTraversalCheckResults _traversalcheckresults)) (.BackLedgeLocation (Utilities|Struct|BreakTraversalCheckResults _traversalcheckresults)) (.BackLedgeNormal (Utilities|Struct|BreakTraversalCheckResults _traversalcheckresults)) (.bHasBackFloor (Utilities|Struct|BreakTraversalCheckResults _traversalcheckresults)) (.BackFloorLocation (Utilities|Struct|BreakTraversalCheckResults _traversalcheckresults)) (.ObstacleHeight (Utilities|Struct|BreakTraversalCheckResults _traversalcheckresults)) (.ObstacleDepth (Utilities|Struct|BreakTraversalCheckResults _traversalcheckresults)) (.BackLedgeHeight (Utilities|Struct|BreakTraversalCheckResults _traversalcheckresults)) (.TraversalActor (Utilities|Struct|BreakTraversalCheckResults _traversalcheckresults)) _asanim_montage (Math|Float|Clamp(Float) (- (.selectedtime (Class|PoseSearchLibrary|MotionMatch AnimInstance (Utilities|Array|MakeArray _aspose_search_database) "PoseHistory")) 0.02) 0.0 (.selectedtime (Class|PoseSearchLibrary|MotionMatch AnimInstance (Utilities|Array|MakeArray _aspose_search_database) "PoseHistory"))) (* (.wantedplayrate (Class|PoseSearchLibrary|MotionMatch AnimInstance (Utilities|Array|MakeArray _aspose_search_database) "PoseHistory")) 0.85 (Variables|Default|GetCurrentTraversalPlayRate)))))
                (CallFunction|PerformTraversal _structout)
                (CallFunction|ServerPerformTraversal _structout))
              (:CastFailed
                (Class|TraversalComponent|TraversalCompleted (Variables|Default|GetTraversalComp))))))))))

(event Input|KeyboardEvents|Escape
  (params (Key :type Key%20Structure :default "None"))
  ;[0.15 0.15 0.15 0.5] Testing
  ;;[0.15 0.15 0.15 0.5] Quit Game (To be Removed)
  (:Pressed
    (Game|QuitGame 0 "Quit" false)))

(event Input|KeyboardEvents|1
  (params (Key :type Key%20Structure :default "None"))
  ;[0.15 0.15 0.15 0.5] Testing
  (:Pressed
    (Utilities|FlowControl|FlipFlop
      (:A
        (Utilities|Time|SetGlobalTimeDilation 0.1))
      (:B
        (Utilities|Time|SetGlobalTimeDilation 1.0)))))

(fn ConstructionScript)