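; Player character Blueprint that plays random idle break animations on the character mesh.
; A native or inherited event calls a server event, which evaluates a Chooser against the main player AnimBP and picks a random montage from the results.
; A multicast event plays that montage, re-runs the idle break timer checks on completion, and clears the idle break flag on blend out, interruption or notify end.
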(event Custom|Server_PlayEvaluateIdleBreak
  ;[0 0 0 0.5] Perform Idle Break
  (bind _asabp_main_player (Utilities|Casting|CastToABP_MainPlayer (Components|SkeletalMesh|GetAnimInstance (Variables|Default|GetCharacterMesh))))
  (bind _result (|EvaluateChooser2 _asabp_main_player)
    (:execute
      (bind _asanim_montage (Utilities|Casting|CastToAnimMontage (Class|PoseSearchDatabase|GetAnimationAsset _result (Math|Random|RandomInteger (Class|PoseSearchDatabase|GetNumAnimationAssets _result)))))
      (CallFunction|MCPlayIdleBreaks _asanim_montage))))

(event Custom|MC_PlayIdleBreaks
  (params (Idle%20Break%20Anim%20Montage :type Anim%20Montage%20Object%20Reference))
  ;[0 0 0 0.5] Perform Idle Break
  (Animation|Montage|PlayMontage (Variables|Default|GetCharacterMesh) Idle%20Break%20Anim%20Montage
    (:OnCompleted
      (Class|PlayerCharacter|PerformIdleBreakTimerChecks))
    (:OnBlendOut
      (Variables|Default|SetbShouldPerformIdleBreak false :!label _label))
    (:OnInterrupted
      (goto _label))
    (:OnNotifyEnd
      (goto _label))))

(event EventBlueprintPerformIdleBreak
  ;[0 0 0 0.5] Perform Idle Break
  (CallFunction|ServerPlayEvaluateIdleBreak))

(fn ConstructionScript)