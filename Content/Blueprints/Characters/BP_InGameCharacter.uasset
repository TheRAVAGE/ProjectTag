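; Playable character Blueprint for a runner/catcher game, handling animation-driven traversal, catches, idle breaks and ragdoll get-ups.
; Choosers select montages or pose search databases, with motion matching refining traversals and multi-character motion matching pairing catcher and target animations.
; Traversal plays locally, then replicates via server and multicast with warp targets; a runner finishing get-up triggers a role swap.
; Temporary debug keys cover slow motion, dummy spawning, role changes and ragdoll.
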(event Custom|Server_PlayEvaluateIdleBreak
  ;[0 0 0 0.5] Perform Idle Break
  (bind _asabp_main_player (Utilities|Casting|CastToABP_MainPlayer (Components|SkeletalMesh|GetAnimInstance (Variables|Default|GetCharacterMesh))))
  (bind _result (|EvaluateChooser2 _asabp_main_player)
    (:execute
      (bind _object (Utilities|AsyncLoadAsset _result)
        (:Completed
          (bind _aspose_search_database (Utilities|Casting|CastToPoseSearchDatabase _object))
          (bind _asanim_montage (Utilities|Casting|CastToAnimMontage (Class|PoseSearchDatabase|GetAnimationAsset _aspose_search_database (Math|Random|RandomInteger (Class|PoseSearchDatabase|GetNumAnimationAssets _aspose_search_database)))))
          (bind _output_get (Variables|Default|SetCurrentlyPlaying_IdleAnimMontage _asanim_montage))
          (CallFunction|MCPlayIdleBreaks _output_get))))))

(event Custom|MC_PlayIdleBreaks
  (params (Idle%20Break%20Anim%20Montage :type Anim%20Montage%20Object%20Reference))
  ;[0 0 0 0.5] Perform Idle Break
  (Animation|Montage|PlayMontage (Variables|Default|GetCharacterMesh) Idle%20Break%20Anim%20Montage
    (:OnCompleted
      (Class|PlayerCharacter|ServerPerformIdleBreakTimerChecks)
      (Variables|Default|SetbShouldPerformIdleBreak false))
    (:OnBlendOut
      (Variables|Default|SetbShouldPerformIdleBreak false :!label _label))
    (:OnInterrupted
      (goto _label))
    (:OnNotifyEnd
      (goto _label))))

(event Custom|MC_PerformTraversal
  (params (TraversalCheckResults :type Traversal%20Check%20Results%20Structure))
  ;[0.15 0.005283 0 0.5] Traversal
  (if (not (Pawn|IsLocallyControlled))
    (CallFunction|PerformTraversal TraversalCheckResults)))

(event Custom|Server_PerformTraversal
  (params (TraversalCheckResults :type Traversal%20Check%20Results%20Structure))
  ;[0.15 0.005283 0 0.5] Traversal
  (CallFunction|MCPerformTraversal TraversalCheckResults))

(event Custom|PerformTraversal
  (params (TraversalCheckResults :type Traversal%20Check%20Results%20Structure))
  (bind (_traversalactor _chosenmontage _starttime _playrate) (Utilities|Struct|BreakTraversalCheckResults TraversalCheckResults))
  (bind _traversalcomp (Variables|Default|GetTraversalComp))
  (bind _charactermovementcomp (Variables|Default|GetCharacterMovementComp))
  (bind _capsulecomp (Variables|Default|GetCapsuleComp))
  ;[0.15 0.005283 0 0.5] Traversal
  (Animation|Montage|PlayMontage (Variables|Default|GetCharacterMesh) _chosenmontage _playrate _starttime
    (:then
      (Class|TraversalComponent|SetWarpTargetsforTraversal _traversalcomp TraversalCheckResults)
      (Pawn|Components|CharacterMovement|SetMovementMode _charactermovementcomp "MOVE_Flying" 0)
      (Class|PlayerCharacter|SetReplicationBehaviour true)
      (Collision|IgnoreActorwhenMoving _capsulecomp _traversalactor true)
      (Class|PlayerCharacter|ServerAddGameplayTag "(TagName=\"Tag.Player.Status.Action.Traversal\")")
      (Class|TraversalInterface|SetTraversingCharacter(Message) _traversalactor self))
    (:OnCompleted
      (Class|TraversalComponent|RemoveWarpTargetsforTraversal _traversalcomp :!label _label)
      (Pawn|Components|CharacterMovement|SetMovementMode _charactermovementcomp "MOVE_Walking" 0)
      (Class|PlayerCharacter|SetReplicationBehaviour false)
      (Collision|ClearMoveIgnoreActors _capsulecomp)
      (Class|TraversalComponent|TraversalCompleted (Variables|Default|GetTraversalComp))
      (Class|PlayerCharacter|ServerRemoveGameplayTag "(TagName=\"Tag.Player.Status.Action.Traversal\")" false)
      (Class|TraversalInterface|SetTraversingCharacter(Message) _traversalactor))
    (:OnBlendOut
      (goto _label))
    (:OnInterrupted
      (goto _label))))

(event Custom|Server_ChangeRole
  (bind _returnvalue (Game|GetGameMode))
  (bind _rolemanagercomp (Variables|Default|GetRoleManagerComp))
  ;[0.15 0.15 0.15 0.5] Testing
  ;;[0.15 0.15 0.15 0.5] Test - Change Role
  (switch Utilities|FlowControl|Switch|SwitchonERoleType (Variables|/Script/ProjectTag.RoleManagerComponent|GetCurrentRole (Variables|Default|GetRoleManagerComp))
    (:E_Runner
      (Class|RoleManagerComponent|ServerRoleChanged _rolemanagercomp _returnvalue "E_Catcher"))
    (:E_Catcher
      (Class|RoleManagerComponent|ServerRoleChanged _rolemanagercomp _returnvalue "E_Runner"))))

(event Custom|Server_SpawnTestDummy
  (params (Location :type Vector))
  ;[0.15 0.15 0.15 0.5] Testing
  ;;[0.15 0.15 0.15 0.5] Spawn Test Dummy
  (bind _returnvalue (AI|SpawnAIFromClass "BP_InGameCharacter_C" 0 Location "0, 0, 0" false 0))
  (bind _asmain_player_character (Utilities|Casting|CastToMain_PlayerCharacter _returnvalue))
  (Class|TagCharacterInterface|ServerAssignRole _asmain_player_character (Game|GetGameMode) "E_Runner"))

(event EventBlueprintPerformIdleBreak
  ;[0 0 0 0.5] Perform Idle Break
  (CallFunction|ServerPlayEvaluateIdleBreak))

(event EventBlueprintEvaluateTraversal
  (params (AnimInstance :type Main%20Anim%20Instance%20Object%20Reference) (TraversalCheckResults :type Traversal%20Check%20Results%20Structure))
  ;[0.15 0.005283 0 0.5] Traversal
  (if (Pawn|IsLocallyControlled)
    (bind (_traversalcheckresults _result) (|EvaluateChooser2 AnimInstance TraversalCheckResults)
      (:execute
        (bind _object (Utilities|AsyncLoadAsset _result)
          (:Completed
            (bind _aspose_search_database (Utilities|Casting|CastToPoseSearchDatabase _object))
            (bind _asanim_montage (Utilities|Casting|CastToAnimMontage (.selectedanim (Class|PoseSearchLibrary|MotionMatch AnimInstance (Utilities|Array|MakeArray _aspose_search_database) "PoseHistory")))
              (:then
                (bind _structout (Utilities|Struct|SetmembersinTraversalCheckResults (Utilities|Struct|MakeTraversalCheckResults (.TraversableType (Utilities|Struct|BreakTraversalCheckResults _traversalcheckresults)) (.DistanceToTraversalObject (Utilities|Struct|BreakTraversalCheckResults _traversalcheckresults)) (.bHasFrontLedge (Utilities|Struct|BreakTraversalCheckResults _traversalcheckresults)) (.FrontLedgeLocation (Utilities|Struct|BreakTraversalCheckResults _traversalcheckresults)) (.FrontLedgeNormal (Utilities|Struct|BreakTraversalCheckResults _traversalcheckresults)) (.bHasBackLedge (Utilities|Struct|BreakTraversalCheckResults _traversalcheckresults)) (.BackLedgeLocation (Utilities|Struct|BreakTraversalCheckResults _traversalcheckresults)) (.BackLedgeNormal (Utilities|Struct|BreakTraversalCheckResults _traversalcheckresults)) (.bHasBackFloor (Utilities|Struct|BreakTraversalCheckResults _traversalcheckresults)) (.BackFloorLocation (Utilities|Struct|BreakTraversalCheckResults _traversalcheckresults)) (.ObstacleHeight (Utilities|Struct|BreakTraversalCheckResults _traversalcheckresults)) (.ObstacleDepth (Utilities|Struct|BreakTraversalCheckResults _traversalcheckresults)) (.BackLedgeHeight (Utilities|Struct|BreakTraversalCheckResults _traversalcheckresults)) (.TraversalActor (Utilities|Struct|BreakTraversalCheckResults _traversalcheckresults)) _asanim_montage (Math|Float|Clamp(Float) (- (.selectedtime (Class|PoseSearchLibrary|MotionMatch AnimInstance (Utilities|Array|MakeArray _aspose_search_database) "PoseHistory")) 0.02) 0.0 (.selectedtime (Class|PoseSearchLibrary|MotionMatch AnimInstance (Utilities|Array|MakeArray _aspose_search_database) "PoseHistory"))) (* (.wantedplayrate (Class|PoseSearchLibrary|MotionMatch AnimInstance (Utilities|Array|MakeArray _aspose_search_database) "PoseHistory")) 0.85 (Variables|Default|GetCurrentTraversalPlayRate)))))
                (CallFunction|PerformTraversal _structout)
                (CallFunction|ServerPerformTraversal _structout))
              (:CastFailed
                (Class|TraversalComponent|TraversalCompleted (Variables|Default|GetTraversalComp))))))))))

(event EventTryRagdollGetup
  ;[0.15 0.05386 0.000193] Get Up - From Ragdoll
  (bind _returnvalue (Components|SkeletalMesh|GetAnimInstance (Variables|Default|GetCharacterMesh)))
  (Class|AnimInstance|SavePoseSnapshot _returnvalue "Ragdoll")
  (Class|PoseSearchLibrary|OverridePoseHistoryfromOwningMesh _returnvalue "PoseHistory")
  (bind _returnvalue_2 (Class|MainAnimInstance|GetPoseHistory (Variables|Default|GetPlayerAnimInstance)))
  (bind (_s_cht_getupmontage_out _result) (|EvaluateChooser2 (Utilities|Struct|MakeS_CHT_GetUpMontage_IN _returnvalue_2 (Class|PlayerCharacter|RagdollPlayRollingGetup) "E_Stand"))
    (:execute
      (Animation|Montage|PlayMontage (Variables|Default|GetCharacterMesh) _result 1.0 (Utilities|Struct|BreakS_CHT_GetUpMontage_OUT _s_cht_getupmontage_out)
        (:then
          (Class|PhysicsControlComponent|SetControlDatasinSet (Variables|Default|GetPhysicsControlComp) "ParentSpace" (Utilities|Struct|MakePhysicsControlData true 0.0 1.0 0.0 0.0 0.0 1.0 0.0 0.0 0.0 0.0))
          (Utilities|FlowControl|Delay 0.2)
          (Class|MainPlayerCharacter|ApplyRagdollPhysics false))
        (:OnCompleted
          (if (and (Ability|HasAuthority) (Utilities|Enum|Equal(Enum) (Class|MainPlayerCharacter|GetCurrentRole) "E_Runner")) :!label _label
            (bind _returnvalue_3 (Class|TagCharacterInterface|GetPlayerCharacter (Variables|Default|GetCatcherInterface)))
            (Class|MainPlayerCharacter|ServerSwapRoles _returnvalue_3)))
        (:OnBlendOut
          (goto _label))))))

(event Input|KeyboardEvents|Escape
  (params (Key :type Key%20Structure :default "None"))
  ;[0.15 0.15 0.15 0.5] Testing
  ;;[0.15 0.15 0.15 0.5] Quit Game (To be Removed)
  (:Pressed
    (Game|QuitGame 0 "Quit" false)))

(event Input|KeyboardEvents|2
  (params (Key :type Key%20Structure :default "None"))
  ;[0.15 0.15 0.15 0.5] Testing
  ;;[0.15 0.15 0.15 0.5] Test - Change Role
  (:Pressed
    (CallFunction|ServerChangeRole)))

(event Input|KeyboardEvents|1
  (params (Key :type Key%20Structure :default "None"))
  ;[0.15 0.15 0.15 0.5] Testing
  ;;[0.15 0.15 0.15 0.5] Slow Mo Test
  (:Pressed
    (Utilities|FlowControl|FlipFlop
      (:A
        (Utilities|Time|SetGlobalTimeDilation 0.1))
      (:B
        (Utilities|Time|SetGlobalTimeDilation 1.0)))))

(event Input|KeyboardEvents|CtrlR
  (params (Key :type Key%20Structure :default "None"))
  ;[0.15 0.15 0.15 0.5] Testing
  ;;[0.15 0.15 0.15 0.5] Spawn Test Dummy
  (:Pressed
    (CallFunction|ServerSpawnTestDummy (+ (+ (Transformation|GetActorLocation) (* (Transformation|GetActorForwardVector) 4e+02)) "0.000000,0.000000,20.000000"))))

(event Input|KeyboardEvents|R
  (params (Key :type Key%20Structure :default "None"))
  ;[0.15 0.15 0.15 0.5] Testing
  ;;[0.15 0.15 0.15 0.5] Trigger Ragdoll
  (:Pressed
    (Class|MainPlayerCharacter|TriggerRagDoll true (Utilities|Struct|MakeMontageBlendSettings))))

(event Input|KeyboardEvents|3
  (params (Key :type Key%20Structure :default "None"))
  (bind _returnvalue (Utilities|String|MakeLiteralString "Remaining Match Time"))
  ;[0.15 0.15 0.15 0.5] Testing
  (:Pressed
    (bind _asmain_level_game_mode (Utilities|Casting|CastToMainLevel_GameMode (Game|GetGameMode)))
    (Development|PrintString (Utilities|String|Append _returnvalue " : " (Utilities|String|ToString(Integer) (Variables|/Script/ProjectTag.MainLevel_GameMode|GetRemainingMatchTime _asmain_level_game_mode))) true true "(R=0.000000,G=0.660000,B=1.000000,A=1.000000)" 5.0 (Utilities|String|StringToName _returnvalue))))

(fn ConstructionScript)

(fn EvaluateCatchAttempt
  (params (TargetPlayerInterface :type Tag%20Character%20Interface%20Interface%20%28by%20ref%29) (Speed :type Float%20%28single-precision%29))
  (bind _mmcatchresults (|CallParentFunction TargetPlayerInterface Speed))
  (LocalVariables|SetMMMulti%20Catch%20Results _mmcatchresults)
  (Utilities|FlowControl|Sequence
    (:then_0
      ;[0.15 0.15 0.15 0.5] Evaluating Chooser
      (bind (_s_cht_interactionspsd_out _result) (|EvaluateChooser2 (Utilities|Struct|MakeS_CHT_InteractionsPSD_IN Speed))
        (:execute
          (LocalVariables|SetChooser%20Outputs _s_cht_interactionspsd_out)
          (LocalVariables|SetChooser%20Results _result))))
    (:then_1
      ;[0.15 0.15 0.15 0.5] Declaring and empty query
      (bind _structout (Utilities|Struct|SetmembersinPoseSearchMotionMatchMultiQuery (Utilities|Struct|MakePoseSearchMotionMatchMultiQuery (LocalVariables|GetChooser%20Results))))
      (LocalVariables|SetMMMulti%20Query _structout)
      ;[0.15 0.15 0.15 0.5] Assign Role for Catcher
      (Utilities|Array|Add (.animcontextsroles (LocalVariables|GetMMMulti%20Query)) (Utilities|Struct|MakePoseSearchAnimContextRoles (Variables|Default|GetPlayerAnimInstance) (.initiatorroles (LocalVariables|GetChooser%20Outputs))))
      ;[0.15 0.15 0.15 0.5] Assign Role for Target
      (if (Utilities|IsValidInterface TargetPlayerInterface)
        (bind _returnvalue (Class|TagCharacterInterface|GetAnimInstance TargetPlayerInterface))
        (Utilities|Array|Add (.animcontextsroles (LocalVariables|GetMMMulti%20Query)) (Utilities|Struct|MakePoseSearchAnimContextRoles _returnvalue (.targetroles (LocalVariables|GetChooser%20Outputs))))
        (else
          (Development|PrintString "Invalid Interface"))))
    (:then_3
      ;[0.15 0.15 0.15 0.5] Motion Match Multi
      (bind _results (Class|PoseSearchInteractionLibrary|MotionMatchMulti (Utilities|Array|MakeArray (LocalVariables|GetMMMulti%20Query)) "PoseHistory"))
      (bind _output_get (LocalVariables|SetMMMulti%20Catch%20Results _results))
      ;[0.15 0.15 0.15 0.5] Triggering Animations
      (for _array_element _output_get
        (bind _asmain_player_character (Utilities|Casting|CastToMain_PlayerCharacter (Class|PoseSearchLibrary|GetActor _array_element)))
        (Class|MainPlayerCharacter|MCPerformCatchAnimMontages _asmain_player_character _array_element self)))
    (:then_4
      (return (LocalVariables|GetMMMulti%20Catch%20Results)))))

(fn BPApplyRagdollPhysics
  (params (bShouldApplyPhysics :type Boolean))
  (bind _ragdoll_leftleg (Variables|Default|GetRagDoll_LeftLeg))
  (bind _ragdoll_rightleg (Variables|Default|GetRagDoll_RightLeg))
  (bind _charactermesh (Variables|Default|GetCharacterMesh))
  (if bShouldApplyPhysics
    (bind _returnvalue (Class|PhysicsControlBPLibrary|EnableCollisionBetweenBodyArrays _charactermesh _ragdoll_leftleg _charactermesh _ragdoll_rightleg))
    (return _returnvalue)
    (else
      (bind _returnvalue_2 (Class|PhysicsControlBPLibrary|DisableCollisionBetweenBodyArrays _charactermesh _ragdoll_leftleg _charactermesh _ragdoll_rightleg))
      (return _returnvalue_2))))