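; BP_TraversableBase is a base Blueprint for traversable world objects that exposes ledge data for traversal.
; Its construction script gathers four ledge components into SplineCollections.
; It also builds LedgeMap, a two-way lookup pairing Ledge01 with Ledge02 and Ledge03 with Ledge04, so each ledge resolves to its counterpart.
; The event graph holds no runtime logic.
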(event EventBeginPlay)

(event Collision|EventActorBeginOverlap
  (params (OtherActor :type Actor%20Object%20Reference)))

(event EventTick
  (params (DeltaSeconds :type Float%20%28single-precision%29)))

(fn ConstructionScript
  (Variables|Default|SetSplineCollections (Utilities|Array|MakeArray (Variables|Default|GetLedge%2001) (Variables|Default|GetLedge%2002) (Variables|Default|GetLedge%2003) (Variables|Default|GetLedge%2004)))
  (Variables|Default|SetLedgeMap (Utilities|Map|MakeMap (Variables|Default|GetLedge%2001) (Variables|Default|GetLedge%2002) (Variables|Default|GetLedge%2002) (Variables|Default|GetLedge%2001) (Variables|Default|GetLedge%2003) (Variables|Default|GetLedge%2004) (Variables|Default|GetLedge%2004) (Variables|Default|GetLedge%2003))))